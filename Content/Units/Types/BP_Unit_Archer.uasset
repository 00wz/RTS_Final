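; BP_Unit_Archer is an archer unit type that attacks by shooting arrows.
; Its Attack override runs the parent attack, then, if the target is valid, spawns a BP_Arrow at the archer's location.
; The arrow receives a snapshot of the target's location at spawn, not a reference to the target actor.
; Everything else is left to the parent class, as the event graph holds only disabled stubs.
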(event EventBeginPlay
  (|CallParentFunction) ; This node is disabled and will not be called.\nDrag off pins to build functionality.
)

(event Collision|EventActorBeginOverlap
  (params (OtherActor :type Actor%20Object%20Reference))
  (|CallParentFunction OtherActor) ; This node is disabled and will not be called.\nDrag off pins to build functionality.
)

(event EventTick
  (params (DeltaSeconds :type Float%20%28single-precision%29))
  (|CallParentFunction DeltaSeconds) ; This node is disabled and will not be called.\nDrag off pins to build functionality.
)

(fn ConstructionScript
  (|CallParentFunction))

(fn Attack
  (params (Target :type BP%20Unit%20Base%20Object%20Reference))
  (|CallParentFunction Target)
  (Utilities|IsValid Target
    (:Is%20Valid
      (Game|SpawnActorfromClass "/Game/Units/VFX/BP_Arrow.BP_Arrow_C" (Math|Transform|MakeTransform (Transformation|GetActorLocation) "0, 0, 0" "1,1,1") "Undefined" 0 (Transformation|GetActorLocation Target) 0))))