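; Base RTS unit character with health, team, selection outline and combat.
; Move and attack orders write to the AI blackboard, FindTarget returns the first living enemy within detection radius, and Attack plays a random montage while applying damage immediately.
; Health changes update a team-colored bar widget.
; Death notifies BP_GM_RTS, stops AI and movement, then freezes a random death animation on a timer just before it ends.
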(event EventBeginPlay
  (CallFunction|InitHealthBar)
  (Variables|Default|SetCurrenHealth (Variables|Stats|GetMaxHealth)))

(event Collision|EventActorBeginOverlap
  (params (OtherActor :type Actor%20Object%20Reference)))

(event EventTick
  (params (DeltaSeconds :type Float%20%28single-precision%29))
  (CallFunction|RotatetoDirection DeltaSeconds))

(event EventOrderMove
  (params (Location :type Vector :default "0, 0, 0"))
  (AI|Components|Blackboard|SetValueasVector (AI|GetBlackboard self) (Variables|BlackboardValues|GetMoveLocationKey) Location))

(event EventOrderAttack
  (params (Target :type Actor%20Object%20Reference))
  (AI|Components|Blackboard|SetValueasObject (AI|GetBlackboard self) (Variables|BlackboardValues|GetTargetActorKey) Target))

(fn ConstructionScript)

(fn TakeDamage
  (params (Damage :type Float%20%28single-precision%29))
  (bind _output_get (Variables|Default|SetCurrenHealth (- (Variables|Default|GetCurrenHealth) Damage)))
  (CallFunction|RefreshWidget)
  (if (<= _output_get 0.0)
    (CallFunction|Die)))

(fn Die
  (if (not (Variables|Default|GetIsDead))
    (Utilities|FlowControl|Sequence
      (:then_0
        (bind _asbp_gm_rts (Utilities|Casting|CastToBP_GM_RTS (Game|GetGameMode)))
        (Default|OnUnitDied _asbp_gm_rts self)
        (Variables|Default|SetIsDead true)
        (CallFunction|SetSelected false)
        (Rendering|SetVisibility (Variables|Default|GetWidget) false false))
      (:then_1
        (AI|Logic|StopLogic (Variables|/Script/AIModule.AIController|GetBrainComponent (AI|GetAIController self)) "")
        (Pawn|Components|CharacterMovement|DisableMovement (Variables|Character|GetCharacterMovement)))
      (:then_2
        (bind _returnvalue (Class|AnimInstance|PlaySlotAnimation (Components|SkeletalMesh|GetAnimInstance (Variables|Character|GetMesh)) (.OutItem (Utilities|Array|Random (Variables|Default|GetDeathAnimations))) "DefaultSlot" 0.05 0.05 1.0 1))
        (Utilities|Time|SetTimerbyFunctionName self "FreezAnimations" (* _returnvalue 0.95))))))

(fn RefreshWidget
  (bind _aswbp_health_bar (Utilities|Casting|CastToWBP_HealthBar (UserInterface|GetWidget (Variables|Default|GetWidget))))
  (Variables|/Game/UI/Widgets/WBP_HealthBar.WBP_HealthBar_C|SetPercent _aswbp_health_bar (/ (Variables|Default|GetCurrenHealth) (Variables|Stats|GetMaxHealth))))

(fn InitHealthBar
  (bind _aswbp_health_bar (Utilities|Casting|CastToWBP_HealthBar (UserInterface|GetWidget (Variables|Default|GetWidget))))
  (Utilities|FlowControl|Sequence
    (:then_0
      (Default|SetBarColor _aswbp_health_bar (Math|Conversions|ToColor(LinearColor) (Utilities|Select :Index (Variables|Default|GetTeam) :Option%200 (Class|KismetMathLibrary|LinearColorGreen) :Option%201 (Class|KismetMathLibrary|LinearColorRed)))))
    (:then_1
      (Default|SetBarWidth _aswbp_health_bar (Variables|Stats|GetMaxHealth)))))

(fn SetSelected
  (params (Value :type Boolean))
  (Rendering|SetRenderCustomDepth (Variables|Character|GetMesh) Value))

(fn Attack
  (params (Target :type BP%20Unit%20Base%20Object%20Reference))
  (Utilities|FlowControl|Sequence
    (:then_0
      (Class|AnimInstance|PlaySlotAnimation (Components|SkeletalMesh|GetAnimInstance (Variables|Character|GetMesh)) (.OutItem (Utilities|Array|Random (Variables|Default|GetAttackAnimations))) "DefaultSlot" 0.05 0.05 1.0 1))
    (:then_1
      (CallFunction|TakeDamage Target (Variables|Stats|GetDamage)))))

(fn FreezAnimations
  (Variables|/Script/Engine.SkeletalMeshComponent|SetGlobalAnimRateScale (Variables|Character|GetMesh) 0.0))

(fn TakeHealth
  (params (Value :type Float%20%28single-precision%29))
  (Variables|Default|SetCurrenHealth (Math|Float|Min(Float) (+ (Variables|Default|GetCurrenHealth) Value) (Variables|Stats|GetMaxHealth)))
  (CallFunction|RefreshWidget))

(fn FindTarget
  (Utilities|FlowControl|Sequence
    (:then_0
      (bind _outactors (Actor|GetAllActorsOfClass "BP_UnitBase_C"))
      (bind _array_element (Utilities|Array|ForEachLoopwithBreak _outactors)
        (:LoopBody
          (if (Math|Boolean|ANDBoolean (not (Variables|BP_UnitBase_C|GetIsDead _array_element)) (!= (Variables|BP_UnitBase_C|GetTeam _array_element) (Variables|Default|GetTeam)) (<= (Transformation|GetDistanceTo _array_element self) (Variables|Default|GetDetection%20radius)))
            (return _array_element)))))
    (:then_1
      (return 0))))

(fn RotatetoDirection
  (params (DeltaTime :type Float%20%28single-precision%29))
  (bind _returnvalue (Transformation|GetVelocity))
  (Transformation|SetActorRotation (Class|KismetMathLibrary|RInterptoConstant (Transformation|GetActorRotation) (Math|Rotator|FindLookatRotation (Math|Vector|MakeVector 0.0 0.0 0.0) (Math|Vector|MakeVector (.x _returnvalue) (.y _returnvalue) 0.0)) DeltaTime 7.2e+02)))