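; BP_Arrow is a unit VFX projectile actor that flies in a straight line from its spawn point to a target position.
; On BeginPlay it records its start location and rotates to face the target.
; Tick advances a normalized alpha over the total move time and lerps the location without sweeping.
; On arrival it deactivates the particle system, then destroys itself after a short delay.
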(event EventBeginPlay
  (bind _output_get (Variables|Default|SetStartPosition (Transformation|GetActorLocation)))
  (Transformation|SetActorRotation (Math|Rotator|FindLookatRotation _output_get (Variables|Default|GetTargetPosition))))

(event EventTick
  (params (DeltaSeconds :type Float%20%28single-precision%29))
  (if (not (Variables|Default|GetbPendingKill))
    (bind _output_get (Variables|Default|SetAlpha (+ (/ DeltaSeconds (Variables|Default|GetTotalMoveTime)) (Variables|Default|GetAlpha))))
    (if (>= _output_get 1.0)
      (Variables|Default|SetbPendingKill true)
      (Components|Activation|Deactivate (Variables|Default|GetParticleSystem))
      (Utilities|FlowControl|Delay 2.0)
      (Actor|DestroyActor)
      (else
        (Transformation|SetActorLocation (Math|Vector|Lerp(Vector) (Variables|Default|GetStartPosition) (Variables|Default|GetTargetPosition) (Variables|Default|GetAlpha)) false false)))))

(fn ConstructionScript)