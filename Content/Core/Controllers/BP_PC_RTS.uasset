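; RTS player controller that handles unit selection, orders and the pause menu.
; Left-drag starts the HUD's selection rectangle; each tick while dragging, selection is rebuilt from the HUD's units, keeping only living Team 0 units.
; Right-click traces under the cursor, ordering selected units to attack a Team 1 unit or otherwise move to that point.
; Escape or P opens the in-game menu and pauses the game.
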(event EventBeginPlay
  (bind _asbp_hud_rts (Utilities|Casting|CastToBP_HUD_RTS (HUD|GetHUD)))
  (Variables|Default|SetBP%20HUD%20RTS _asbp_hud_rts))

(event EventTick
  (params (DeltaSeconds :type Float%20%28single-precision%29))
  (Utilities|FlowControl|Sequence
    (:then_0
      (if (Variables|Default|GetbIsDrawning)
        (CallFunction|UpdateUnitsSelection (Variables|/Game/UI/BP_HUD_RTS.BP_HUD_RTS_C|GetSelectedUnits (Variables|Default|GetBP%20HUD%20RTS)))))))

(event Input|MouseEvents|LeftMouseButton
  (params (Key :type Key%20Structure :default "None"))
  (:Pressed
    (Default|StartSelectionRectangleDrawning (Variables|Default|GetBP%20HUD%20RTS))
    (Variables|Default|SetbIsDrawning true))
  (:Released
    (Default|StopSelectionRectangleDrawning (Variables|Default|GetBP%20HUD%20RTS))
    (Variables|Default|SetbIsDrawning false)
    (Development|PrintString (Utilities|String|ToString(Integer) (Utilities|Array|Length (Variables|Default|GetSelectedUnits))))))

(event Input|MouseEvents|RightMouseButton
  (params (Key :type Key%20Structure :default "None"))
  (bind _hitresult (Game|Player|GetHitResultUnderCursorbyChannel "TraceTypeQuery2" true))
  (:Pressed
    (bind _asbp_unit_base (Utilities|Casting|CastToBP_UnitBase (.hitactor _hitresult))
      (:then
        (if (== (Variables|/Game/Units/Base/BP_UnitBase.BP_UnitBase_C|GetTeam _asbp_unit_base) 1)
          (for _array_element (Variables|Default|GetSelectedUnits)
            (Utilities|IsValid _array_element
              (:Is%20Valid
                (Default|OrderAttack _array_element _asbp_unit_base))))
          (else
            (for _array_element_2 (Variables|Default|GetSelectedUnits) :!label _label
              (Utilities|IsValid _array_element_2
                (:Is%20Valid
                  (Default|OrderMove _array_element_2 (.location _hitresult))))))))
      (:CastFailed
        (goto _label)))))

(event Input|KeyboardEvents|Escape
  (params (Key :type Key%20Structure :default "None"))
  (:Pressed
    (bind _returnvalue (UserInterface|CreateWidget "/Game/UI/Widgets/WBP_InGameMenu.WBP_InGameMenu_C"))
    (UserInterface|Viewport|AddtoViewport _returnvalue 0)
    (Game|SetGamePaused true)))

(event Input|KeyboardEvents|P
  (params (Key :type Key%20Structure :default "None"))
  (:Pressed
    (bind _returnvalue (UserInterface|CreateWidget "/Game/UI/Widgets/WBP_InGameMenu.WBP_InGameMenu_C"))
    (UserInterface|Viewport|AddtoViewport _returnvalue 0)
    (Game|SetGamePaused true)))

(fn ConstructionScript)

(fn UpdateUnitsSelection
  (params (Selected :type Array%20of%20BP%20Unit%20Base%20Object%20References))
  (Utilities|FlowControl|Sequence
    (:then_0
      (for _array_element (Variables|Default|GetSelectedUnits)
        (Utilities|IsValid _array_element
          (:Is%20Valid
            (Default|SetSelected _array_element false))))
      (Utilities|Array|Clear (Variables|Default|GetSelectedUnits)))
    (:then_1
      (for _array_element_2 Selected
        (Utilities|IsValid _array_element_2
          (:Is%20Valid
            (if (and (== (Variables|/Game/Units/Base/BP_UnitBase.BP_UnitBase_C|GetTeam _array_element_2) 0) (not (Variables|/Game/Units/Base/BP_UnitBase.BP_UnitBase_C|GetIsDead _array_element_2)))
              (Utilities|Array|Add (Variables|Default|GetSelectedUnits) _array_element_2)
              (Default|SetSelected _array_element_2 true))))))))