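; Camera pawn meant to pan when the mouse nears the viewport edges, currently inactive.
; ProcessCameraControl compares the scaled mouse position to an edge margin and calls MoveInDirection along the root's forward or right vectors.
; MoveInDirection offsets the actor by speed and delta time, without sweep.
; Tick only calls the empty ClampLocationInside stub; ProcessCameraControl is disconnected, so the pawn never moves itself.
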(event EventBeginPlay)

(event Collision|EventActorBeginOverlap
  (params (OtherActor :type Actor%20Object%20Reference)))

(event EventTick
  (params (DeltaSeconds :type Float%20%28single-precision%29))
  (Utilities|FlowControl|Sequence
    (:then_1
      (CallFunction|ClampLocationInside))))

(fn ConstructionScript)

(fn ProcessCameraControl
  (params (DeltaTime :type Float%20%28single-precision%29))
  (bind _returnvalue (Viewport|GetViewportSize))
  (bind _returnvalue_2 (Class|WidgetLayoutLibrary|GetMousePositiononViewport))
  (Utilities|FlowControl|Sequence
    (:then_0
      (if (< (.x (* _returnvalue_2 (Class|WidgetLayoutLibrary|GetViewportScale))) (Variables|Default|GetEdgeMargin))
        (CallFunction|MoveinDirection (Math|Vector|NegateVector (Math|Vector|GetRightVector (Variables|Default|GetDefaultSceneRoot))) DeltaTime)))
    (:then_1
      (if (> (.x (* _returnvalue_2 (Class|WidgetLayoutLibrary|GetViewportScale))) (- (.x _returnvalue) (Variables|Default|GetEdgeMargin)))
        (CallFunction|MoveinDirection (Math|Vector|GetRightVector (Variables|Default|GetDefaultSceneRoot)) DeltaTime)))
    (:then_2
      (if (< (.y (* _returnvalue_2 (Class|WidgetLayoutLibrary|GetViewportScale))) (Variables|Default|GetEdgeMargin))
        (CallFunction|MoveinDirection (Math|Vector|GetForwardVector (Variables|Default|GetDefaultSceneRoot)) DeltaTime)))
    (:then_3
      (if (> (.y (* _returnvalue_2 (Class|WidgetLayoutLibrary|GetViewportScale))) (- (.y _returnvalue) (Variables|Default|GetEdgeMargin)))
        (CallFunction|MoveinDirection (Math|Vector|NegateVector (Math|Vector|GetForwardVector (Variables|Default|GetDefaultSceneRoot))) DeltaTime)))))

(fn MoveinDirection
  (params (Direction :type Vector) (DeltaTime :type Float%20%28single-precision%29))
  (Transformation|AddActorWorldOffset (* (* Direction (Variables|Default|GetMoveSpeed)) DeltaTime)))

(fn ClampLocationInside)