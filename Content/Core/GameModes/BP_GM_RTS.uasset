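; RTS game mode that tracks living units per side and ends the match when one side is wiped out.
; On BeginPlay it counts BP_UnitBase actors, treating team 0 as the player and every other team as enemies.
; OnUnitDied decrements the matching count, then CheckGameEnd shows the WBP_EndGame widget as defeat or victory, with defeat checked first.
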(event Custom|OnUnitDied
  (params (Sender :type BP%20Unit%20Base%20Object%20Reference))
  (Utilities|FlowControl|Sequence
    (:then_0
      (if (== (Variables|/Game/Units/Base/BP_UnitBase.BP_UnitBase_C|GetTeam Sender) 0)
        (Math|Integer|DecrementInt (Variables|Default|GetPlayerCount))
        (else
          (Math|Integer|DecrementInt (Variables|Default|GetEnemyCount)))))
    (:then_1
      (CallFunction|CheckGameEnd))))

(event EventBeginPlay
  (bind _outactors (Actor|GetAllActorsOfClass "/Game/Units/Base/BP_UnitBase.BP_UnitBase_C"))
  (for _array_element _outactors
    (if (== (Variables|/Game/Units/Base/BP_UnitBase.BP_UnitBase_C|GetTeam _array_element) 0)
      (Math|Integer|IncrementInt (Variables|Default|GetPlayerCount))
      (else
        (Math|Integer|IncrementInt (Variables|Default|GetEnemyCount))))))

(fn ConstructionScript)

(fn CheckGameEnd
  (Utilities|FlowControl|Sequence
    (:then_0
      (if (<= (Variables|Default|GetPlayerCount) 0)
        (CallFunction|ShowEndScreen false)
        (return)))
    (:then_1
      (if (<= (Variables|Default|GetEnemyCount) 0)
        (CallFunction|ShowEndScreen true)
        (return)))))

(fn ShowEndScreen
  (params (IsVictory :type Boolean))
  (bind _returnvalue (UserInterface|CreateWidget "/Game/UI/Widgets/WBP_EndGame.WBP_EndGame_C" (Game|GetPlayerController 0) IsVictory))
  (UserInterface|Viewport|AddtoViewport _returnvalue 10))